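; Paper2D fighter character for a local two-player versus game, with movement, jump, ground and air attacks, and blocking.
; Player one uses Enhanced Input and relays player two's bindings and hard-coded keys to the cached second pawn, which is tinted when flagged.
; PaperZD node jumps play animations, flipbook-length delays lock movement, and separate events damage hitbox overlaps.
; Blocking reduces damage; death disables both players' input and signals the win.
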(event Custom|MovePlayer2
  (params (AxisValue :type Float%20%28double-precision%29))
  (Pawn|Input|AddMovementInput "1.000000,0.000000,0.000000" AxisValue false))

(event Custom|BlockP2
  (if (not (AI|Components|NavMovement|IsFalling (Variables|Character|GetCharacterMovement)))
    (Variables|Default|SetisBlocking true)
    (Variables|/Script/Engine.CharacterMovementComponent|SetMaxWalkSpeed (Variables|Character|GetCharacterMovement) 0.0)))

(event Custom|Attack
  (for _array_element (Collision|GetOverlappingActors (Variables|Default|GetAttackBox) 0 :!class /Script/Engine.PrimitiveComponent)
    (if (!= _array_element self)
      (Game|Damage|ApplyDamage _array_element (Variables|Default|GetBase%20Damage) 0 0))))

(event Custom|LoadControls
  (bind _asplayer_controller (Utilities|Casting|CastToPlayerController (Pawn|GetController)))
  (Utilities|IsValid (PlayerController|LocalPlayerSubsystems|GetEnhancedInputLocalPlayerSubsystem _asplayer_controller)
    (:Is%20Valid
      (Input|AddMappingContext (PlayerController|LocalPlayerSubsystems|GetEnhancedInputLocalPlayerSubsystem _asplayer_controller) "/Game/Controls/Fighting_IMC.Fighting_IMC" 0 "(bIgnoreAllPressedKeysUntilRelease=True,bForceImmediately=False,bNotifyUserSettings=False)")
      (Variables|Default|SetPlayerSpeed (Variables|/Script/Engine.CharacterMovementComponent|GetMaxWalkSpeed (Variables|Character|GetCharacterMovement)))
      (Variables|Default|SetPlayerMaxHealth (Variables|Default|GetPlayerHealth)))))

(event Custom|Player2Jump
  (Utilities|BlockCheck
    (:else
      _)
    (:then
      _))
  (Character|Jump))

(event Custom|Player2Attack
  (Utilities|FlowControl|DoOnce false :!label _label
    (:Completed
      (Utilities|BlockCheck
        (:else
          _)
        (:then
          _))
      (Variables|/Script/Engine.CharacterMovementComponent|SetMaxWalkSpeed (Variables|Character|GetCharacterMovement) 0.0)
      (if (AI|Components|NavMovement|IsFalling (Variables|Character|GetCharacterMovement))
        (Class|PaperZDAnimInstance|JumptoNode (Variables|/Script/PaperZD.PaperZDAnimationComponent|GetAnimInstance (Variables|Default|GetAnimationComponent)) "Air_Atk" "None")
        (Utilities|FlowControl|Delay (- (Class|PaperFlipbookComponent|GetFlipbookLength (Variables|Default|GetSprite)) 0.15))
        (else
          (Class|PaperZDAnimInstance|JumptoNode (Variables|/Script/PaperZD.PaperZDAnimationComponent|GetAnimInstance (Variables|Default|GetAnimationComponent)) "Attack" "None")
          (Utilities|FlowControl|Delay (- (Class|PaperFlipbookComponent|GetFlipbookLength (Variables|Default|GetSprite)) 0.15))))
      (Variables|/Script/Engine.CharacterMovementComponent|SetMaxWalkSpeed (Variables|Character|GetCharacterMovement) (Variables|Default|GetPlayerSpeed))
      (goto _label Reset))))

(event Custom|AirAttack
  (for _array_element (Collision|GetOverlappingActors (Variables|Default|GetAirAttackBox) 0 :!class /Script/Engine.PrimitiveComponent)
    (if (!= _array_element self)
      (Game|Damage|ApplyDamage _array_element (Variables|Default|GetBase%20Damage) 0 0))))

(event Custom|StopBlockP2
  (Variables|Default|SetisBlocking false)
  (Variables|/Script/Engine.CharacterMovementComponent|SetMaxWalkSpeed (Variables|Character|GetCharacterMovement) (Variables|Default|GetPlayerSpeed)))

(event Input|EnhancedActionEvents|EnhancedInputActionMove_IA
  (params (ActionValue :type Float%20%28double-precision%29) (ElapsedSeconds :type Float%20%28double-precision%29) (TriggeredSeconds :type Float%20%28double-precision%29) (InputAction :type Input%20Action%20Object%20Reference :default "/Game/Controls/Move_IA.Move_IA"))
  (Pawn|Input|AddMovementInput "1.000000,0.000000,0.000000" ActionValue false))

(event Input|EnhancedActionEvents|EnhancedInputActionJump_IA
  (params (ActionValue :type Boolean) (ElapsedSeconds :type Float%20%28double-precision%29) (TriggeredSeconds :type Float%20%28double-precision%29) (InputAction :type Input%20Action%20Object%20Reference :default "/Game/Controls/Jump_IA.Jump_IA"))
  (:Started
    (Utilities|BlockCheck
      (:else
        _)
      (:then
        _))
    (Character|Jump))
  (:Completed
    (Character|StopJumping)))

(event Input|EnhancedActionEvents|EnhancedInputActionAtk_IA
  (params (ActionValue :type Boolean) (ElapsedSeconds :type Float%20%28double-precision%29) (TriggeredSeconds :type Float%20%28double-precision%29) (InputAction :type Input%20Action%20Object%20Reference :default "/Game/Controls/Atk_IA.Atk_IA"))
  (:Started
    (Utilities|FlowControl|DoOnce false :!label _label
      (:Completed
        (Utilities|BlockCheck
          (:else
            _)
          (:then
            _))
        (Variables|/Script/Engine.CharacterMovementComponent|SetMaxWalkSpeed (Variables|Character|GetCharacterMovement) 0.0)
        (if (AI|Components|NavMovement|IsFalling (Variables|Character|GetCharacterMovement))
          (Class|PaperZDAnimInstance|JumptoNode (Variables|/Script/PaperZD.PaperZDAnimationComponent|GetAnimInstance (Variables|Default|GetAnimationComponent)) "Air_Atk" "None")
          (Utilities|FlowControl|Delay (- (Class|PaperFlipbookComponent|GetFlipbookLength (Variables|Default|GetSprite)) 0.15))
          (else
            (Class|PaperZDAnimInstance|JumptoNode (Variables|/Script/PaperZD.PaperZDAnimationComponent|GetAnimInstance (Variables|Default|GetAnimationComponent)) "Attack" "None")
            (Utilities|FlowControl|Delay (- (Class|PaperFlipbookComponent|GetFlipbookLength (Variables|Default|GetSprite)) 0.15))))
        (Variables|/Script/Engine.CharacterMovementComponent|SetMaxWalkSpeed (Variables|Character|GetCharacterMovement) (Variables|Default|GetPlayerSpeed))
        (goto _label Reset)))))

(event Input|EnhancedActionEvents|EnhancedInputActionMoveP2_IA
  (params (ActionValue :type Float%20%28double-precision%29) (ElapsedSeconds :type Float%20%28double-precision%29) (TriggeredSeconds :type Float%20%28double-precision%29) (InputAction :type Input%20Action%20Object%20Reference :default "/Game/Controls/MoveP2_IA.MoveP2_IA"))
  (Utilities|IsValid (Variables|Default|Getplayer2)
    (:Is%20Valid
      (CallFunction|MovePlayer2 (Variables|Default|Getplayer2) ActionValue))
    (:Is%20Not%20Valid
      (bind _asplayer_character_bp (Utilities|Casting|CastToPlayerCharacterBP (Game|Player|GetPlayerPawn 1)))
      (bind _output_get (Variables|Default|Setplayer2 _asplayer_character_bp))
      (CallFunction|MovePlayer2 _output_get ActionValue))))

(event Input|EnhancedActionEvents|EnhancedInputActionBlock_IA
  (params (ActionValue :type Boolean) (ElapsedSeconds :type Float%20%28double-precision%29) (TriggeredSeconds :type Float%20%28double-precision%29) (InputAction :type Input%20Action%20Object%20Reference :default "/Game/Controls/Block_IA.Block_IA"))
  (:Started
    (if (not (AI|Components|NavMovement|IsFalling (Variables|Character|GetCharacterMovement)))
      (Variables|Default|SetisBlocking true)
      (Variables|/Script/Engine.CharacterMovementComponent|SetMaxWalkSpeed (Variables|Character|GetCharacterMovement) 0.0)))
  (:Completed
    (Variables|Default|SetisBlocking false)
    (Variables|/Script/Engine.CharacterMovementComponent|SetMaxWalkSpeed (Variables|Character|GetCharacterMovement) (Variables|Default|GetPlayerSpeed))))

(event Input|EnhancedActionEvents|EnhancedInputActionBlockP2_IA
  (params (ActionValue :type Boolean) (ElapsedSeconds :type Float%20%28double-precision%29) (TriggeredSeconds :type Float%20%28double-precision%29) (InputAction :type Input%20Action%20Object%20Reference :default "/Game/Controls/BlockP2_IA.BlockP2_IA"))
  (:Started
    (Utilities|IsValid (Variables|Default|Getplayer2)
      (:Is%20Valid
        (CallFunction|BlockP2 (Variables|Default|Getplayer2)))
      (:Is%20Not%20Valid
        (bind _asplayer_character_bp (Utilities|Casting|CastToPlayerCharacterBP (Game|Player|GetPlayerPawn 1)))
        (bind _output_get (Variables|Default|Setplayer2 _asplayer_character_bp))
        (CallFunction|BlockP2 _output_get))))
  (:Completed
    (Utilities|IsValid (Variables|Default|Getplayer2)
      (:Is%20Valid
        (CallFunction|StopBlockP2 (Variables|Default|Getplayer2)))
      (:Is%20Not%20Valid
        (bind _asplayer_character_bp_2 (Utilities|Casting|CastToPlayerCharacterBP (Game|Player|GetPlayerPawn 1)))
        (bind _output_get_2 (Variables|Default|Setplayer2 _asplayer_character_bp_2))
        (CallFunction|StopBlockP2 _output_get_2)))))

(event EventBeginPlay
  (bind _asplayer_controller (Utilities|Casting|CastToPlayerController (Pawn|GetController)))
  (Utilities|IsValid (PlayerController|LocalPlayerSubsystems|GetEnhancedInputLocalPlayerSubsystem _asplayer_controller)
    (:Is%20Valid
      (Input|AddMappingContext (PlayerController|LocalPlayerSubsystems|GetEnhancedInputLocalPlayerSubsystem _asplayer_controller) "/Game/Controls/Fighting_IMC.Fighting_IMC" 0 "(bIgnoreAllPressedKeysUntilRelease=True,bForceImmediately=False,bNotifyUserSettings=False)")
      (Variables|Default|SetPlayerSpeed (Variables|/Script/Engine.CharacterMovementComponent|GetMaxWalkSpeed (Variables|Character|GetCharacterMovement)))
      (Variables|Default|SetPlayerMaxHealth (Variables|Default|GetPlayerHealth)))))

(event Collision|EventActorBeginOverlap
  (params (OtherActor :type Actor%20Object%20Reference)))

(event EventTick
  (params (DeltaSeconds :type Float%20%28single-precision%29)))

(event Game|Damage|EventAnyDamage
  (params (Damage :type Float%20%28single-precision%29) (DamageType :type Damage%20Type%20Object%20Reference) (InstigatedBy :type Controller%20Object%20Reference) (DamageCauser :type Actor%20Object%20Reference))
  (bind _output_get (Variables|Default|SetPlayerHealth (select (Variables|Default|GetisBlocking) (- (Variables|Default|GetPlayerHealth) (/ Damage 5.0)) (- (Variables|Default|GetPlayerHealth) Damage))))
  (Default|CallUpdateHealth)
  (if (<= _output_get 0.0)
    (Utilities|FlowControl|DoOnce false
      (:Completed
        (Class|PaperZDAnimInstance|JumptoNode (Variables|/Script/PaperZD.PaperZDAnimationComponent|GetAnimInstance (Variables|Default|GetAnimationComponent)) "Death" "None")
        (Input|DisableInput (Game|Player|GetPlayerPawn 0) 0)
        (Default|CallPlayerWins)))
    (elif (not (Variables|Default|GetisBlocking))
      (Class|PaperZDAnimInstance|JumptoNode (Variables|/Script/PaperZD.PaperZDAnimationComponent|GetAnimInstance (Variables|Default|GetAnimationComponent)) "Damaged" "None")
      (Variables|/Script/Engine.CharacterMovementComponent|SetMaxWalkSpeed (Variables|Character|GetCharacterMovement) 0.0)
      (Utilities|FlowControl|RetriggerableDelay (- (Class|PaperFlipbookComponent|GetFlipbookLength (Variables|Default|GetSprite)) 0.3))
      (if (not (Variables|Default|GetisBlocking))
        (Variables|/Script/Engine.CharacterMovementComponent|SetMaxWalkSpeed (Variables|Character|GetCharacterMovement) (Variables|Default|GetPlayerSpeed))))))

(event Input|KeyboardEvents|Up
  (params (Key :type Key%20Structure :default "None"))
  (:Pressed
    (Utilities|IsValid (Variables|Default|Getplayer2)
      (:Is%20Valid
        (CallFunction|Player2Jump (Variables|Default|Getplayer2)))
      (:Is%20Not%20Valid
        (bind _asplayer_character_bp (Utilities|Casting|CastToPlayerCharacterBP (Game|Player|GetPlayerPawn 1)))
        (bind _output_get (Variables|Default|Setplayer2 _asplayer_character_bp))
        (CallFunction|Player2Jump _output_get)))))

(event Input|KeyboardEvents|NumPadOne
  (params (Key :type Key%20Structure :default "None"))
  (:Pressed
    (Utilities|IsValid (Variables|Default|Getplayer2)
      (:Is%20Valid
        (CallFunction|Player2Attack (Variables|Default|Getplayer2)))
      (:Is%20Not%20Valid
        (bind _asplayer_character_bp (Utilities|Casting|CastToPlayerCharacterBP (Game|Player|GetPlayerPawn 1)))
        (bind _output_get (Variables|Default|Setplayer2 _asplayer_character_bp))
        (CallFunction|Player2Attack _output_get)))))

(fn ConstructionScript
  (if (Variables|Default|GetisPlayer2)
    (Sprite|SetSpriteColor (Variables|Default|GetSprite) "(R=1.000000,G=0.391474,B=0.341686,A=1.000000)")))